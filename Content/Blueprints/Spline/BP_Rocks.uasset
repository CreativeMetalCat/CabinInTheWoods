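; BP_Rocks is a spline placement Blueprint that builds a fence-style run of random meshes and posts in its construction script.
; It optionally snaps spline points to the landscape with vertical Visibility traces, then divides the spline by the first mesh's width.
; Each segment gets a randomly flipped, straight-tangent spline mesh, avoiding consecutive repeats.
; A random post mesh at each segment start is rotated along the spline's direction.
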(fn ConstructionScript
  (if (and (Utilities|ValidArray? (Variables|Default|GetFence%20Meshs)) (Utilities|ValidArray? (Variables|Default|GetFence%20Post)))
    (if (Variables|Default|GetSnap%20Points%20to%20Landscape)
      ;[0.07036 0.1651 0.9131] Snap Spline Points to Landscape
      (for _index (range 0 (- (Spline|GetNumberOfSplinePoints (Variables|Default|GetSpline)) 1))
        (bind (_outhit _returnvalue) (Collision|LineTraceByChannel (+ (Spline|GetLocationatSplinePoint (Variables|Default|GetSpline) _index "World") "0, 0,1000.000000") (+ (Spline|GetLocationatSplinePoint (Variables|Default|GetSpline) _index "World") "0, 0,-1000.000000") "TraceTypeQuery1" false 0 "None"))
        (if _returnvalue
          (Spline|SetLocationatSplinePoint (Variables|Default|GetSpline) _index (.Location (Collision|BreakHitResult _outhit)) "World" false))))
    ;[0.1119 0.6724 0.1221] Get Size of First Fence
    (Variables|Default|SetFence%20Size (* (.X (Math|Vector|BreakVector (.BoxExtent (Math|BoxSphereBounds|BreakBoxSphereBounds (StaticMesh|GetBounds (Utilities|Array|Get(acopy) (Variables|Default|GetFence%20Meshs))))))) 2.0))
    ;[1 0.3231 0.05613] Spawn Meshs Across Spline
    (for _index_2 (range 0 (Math|Float|Truncate (/ (Spline|GetSplineLength (Variables|Default|GetSpline)) (Variables|Default|GetFence%20Size))))
      (LocalVariables|SetIndex _index_2)
      (bind _returnvalue_2 (AddComponent|AddSplineMeshComponent true))
      ;;[0.3712 0.1301 0.7913] Makes Sure the same mesh does not repeat if there are more than one mesh options
      (LocalVariables|SetL%20Mesh (Utilities|RandomGet (Variables|Default|GetFence%20Meshs)) :!label _label)
      (if (> (Utilities|Array|Length (Variables|Default|GetFence%20Meshs)) 1)
        (if (== (LocalVariables|GetL%20Mesh) (Variables|Default|GetLast%20Fence%20Mesh))
          (goto _label)
          (else
            _)))
      (Components|StaticMesh|SetStaticMesh _returnvalue_2 (LocalVariables|GetL%20Mesh))
      (Variables|Default|SetLast%20Fence%20Mesh (LocalVariables|GetL%20Mesh))
      (Transformation|AttachComponentToComponent _returnvalue_2 (Variables|Default|GetTopScene) "None" "KeepRelative" "KeepRelative" "KeepRelative" true)
      (bind (_out_start _out_end _t_out) (Utilities|RandomFlipVectors (.Start%20Location (CallFunction|GetSplineLocationsatIndex (LocalVariables|GetIndex))) (.End%20Location (CallFunction|GetSplineLocationsatIndex (LocalVariables|GetIndex)))))
      (SplineMesh|SetStartandEnd _returnvalue_2 _out_start _t_out _out_end _t_out true :!class /Script/Engine.SplineMeshComponent)
      (bind _returnvalue_3 (AddComponent|AddStaticMeshComponent false (Math|Transform|MakeTransform (.Start%20Location (CallFunction|GetSplineLocationsatIndex (LocalVariables|GetIndex))) (|GetPostRotation))))
      (Transformation|AttachComponentToComponent _returnvalue_3 (Variables|Default|GetTopScene) "None" "KeepRelative" "KeepRelative" "KeepRelative" true)
      (Components|StaticMesh|SetStaticMesh _returnvalue_3 (Utilities|RandomGet (Variables|Default|GetFence%20Post))))))

(fn GetSplineLocationsatIndex
  (params (Index :type Integer))
  (return (Spline|GetLocationatDistanceAlongSpline (Variables|Default|GetSpline) (* Index (Variables|Default|GetFence%20Size)) "Local") (Spline|GetLocationatDistanceAlongSpline (Variables|Default|GetSpline) (* (+ Index 1) (Variables|Default|GetFence%20Size)) "Local")))